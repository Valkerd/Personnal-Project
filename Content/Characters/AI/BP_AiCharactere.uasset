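; BP_AiCharactere is an AI character that arms itself with a sword and shield.
; On BeginPlay it spawns Shield_BP and Sword_BP at the left and right hand weapon sockets and snaps them onto the Mesh.
; An early PawnSensing follow-the-player test is unwired: its events are empty, and the AIMoveTo and sight-flag logic never runs.
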(event OnSeePawn(PawnSensing)
  (params (Pawn :type Pawn%20Object%20Reference))
  ;[1 1 1] First test AI to follow the player
)

(event Custom|FollowPlayer
  ;[1 1 1] First test AI to follow the player
)

(event EventBeginPlay
  ;[1 1 1] Attach sword and shield IA
  (bind _returnvalue (Game|SpawnActorfromClass "/Game/Weapon/Shield_BP.Shield_BP_C" (Transformation|GetSocketTransform (Variables|Character|GetMesh) "Hand_l_Weapon" "RTS_World") "Undefined" 0 0))
  (Transformation|AttachComponentToComponent _returnvalue (Variables|Character|GetMesh) "Hand_l_Weapon" "SnapToTarget" "SnapToTarget" "SnapToTarget" true)
  (bind _returnvalue_2 (Game|SpawnActorfromClass "/Game/Weapon/Sword_BP.Sword_BP_C" (Transformation|GetSocketTransform (Variables|Character|GetMesh) "hand_r_Weapon" "RTS_World") "Undefined" 0 0))
  (Transformation|AttachComponentToComponent _returnvalue_2 (Variables|Character|GetMesh) "hand_r_Weapon" "SnapToTarget" "SnapToTarget" "SnapToTarget" true))

(event Collision|EventActorBeginOverlap
  (params (OtherActor :type Actor%20Object%20Reference)))

(event EventTick
  (params (DeltaSeconds :type Float%20%28single-precision%29)))

(fn ConstructionScript)